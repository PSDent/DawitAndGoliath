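; DNG player state that coordinates player pawn initialization when play begins on MainMap.
; The non-authority side calls OnLogin, which increments and prints the game instance's LoadCount.
; The authority side polls every second until LoadCount reaches one less than the PlayerArray size.
; It then has the game instance init player pawns, resets the count and sets the game mode's CurrentPlayerCount from the array size.
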(event `self.ReceiveBeginPlay`
  (bind _returnvalue (`GameplayStatics.GetGameState`))
  (bind _gameinstance (`self.GameInstance`))
  (bind _returnvalue_2 (- (`KismetArrayLibrary.Array_Length` (`GameStateBase.PlayerArray` _returnvalue)) 1))
  (bind _asmy_game_instance_bp (cast `/Game/Blueprints/MyGameInstance_BP` (`GameplayStatics.GetGameInstance`)))
  (set `self.GameInstance` _asmy_game_instance_bp)
  (bind _returnvalue_3 (`GameplayStatics.GetCurrentLevelName` true))
  (if (`KismetStringLibrary.EqualEqual_StrStr` _returnvalue_3 "MainMap")
    (`/Engine/EditorBlueprintResources/ActorMacros.Switch Has Authority`
      (:`Authority`
        (cast `/Game/Blueprints/MyGameStateBase_BP` _returnvalue)
        (if (>= (`MyGameInstance.LoadCount` (`self.GameInstance`)) _returnvalue_2) :!label _label
          (`MyGameInstance.InitPlayersPawn` _gameinstance)
          (set `MyGameInstance.LoadCount` 0 _gameinstance)
          (bind _asdnggame_mode_base_bp (cast `/Game/Blueprints/DNGGameModeBase_BP` (`GameplayStatics.GetGameMode`)))
          (set `DNGGameModeBase.CurrentPlayerCount` (- (* _returnvalue_2 2) 1) _asdnggame_mode_base_bp)
          (else
            (`KismetSystemLibrary.Delay` 1.0)
            (goto _label))))
      (:`Remote`
        (`self.OnLogin`)))))

(event `OnLogin`
  (bind _gameinstance (`self.GameInstance`))
  (bind _output_get (set `MyGameInstance.LoadCount` (+ (`MyGameInstance.LoadCount` _gameinstance) 1) _gameinstance))
  (`KismetSystemLibrary.PrintString` (`KismetStringLibrary.Conv_IntToString` _output_get)))

(fn `UserConstructionScript`)
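; Base player controller Blueprint that handles the game-over screen for an RTS versus FPS match.
; BeginPlay creates a GameSetHUD widget for this controller and adds it to the viewport at a high Z-order.
; ShowGameSetUI forwards the IsRts flag to a custom event, which makes the widget visible and sets its end message to announce an RTS or FPS win.
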(event `self.ReceiveBeginPlay`
  (bind _returnvalue (`|CreateWidget` "/Game/Blueprints/GameSetHUD.GameSetHUD_C" self))
  (bind _output_get (set `self.UserWidget` _returnvalue))
  (`UserWidget.AddToViewport` _output_get 100))

(event `self.ShowGameSetUI`
  (params (isRts :type Boolean))
  (`self.Custom Event_0` self isRts))

(event `Custom Event_0`
  (params (isRts :type Boolean))
  (bind _userwidget (`self.UserWidget`))
  (`Widget.SetVisibility` _userwidget "Visible")
  (bind _asgame_set_hud (cast `/Game/Blueprints/GameSetHUD` _userwidget))
  (if isRts
    (bind _endmessage (`/Game/Blueprints/GameSetHUD.EndMessage` _asgame_set_hud))
    (`TextBlock.SetText` _endmessage "RTS Win!")
    (else
      (`TextBlock.SetText` _endmessage "FPS Win!"))))

(fn `NewFunction_0`)

(fn `UserConstructionScript`)